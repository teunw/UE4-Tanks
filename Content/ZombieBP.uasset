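; Zombie actor Blueprint that drives green zombie flipbook animation through ZombieWalk and ZombieAttack events.
; Walking loops the walk flipbook, scaling its play rate with speed derived from distance moved per frame, mapped between WalkSpeed and RunSpeed.
; Attacking plays the attack flipbook once from the start at normal rate.
; The graph holds only animation logic, with no active BeginPlay, overlap or Tick handling.
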(event `self.ZombieWalk`
  (params (DeltaSeconds :type "Float (single-precision)") (DistanceWalkedThisFrame :type "Vector Structure"))
  (bind _paperflipbook (`self.PaperFlipbook`))
  (`PaperFlipbookComponent.SetFlipbook` _paperflipbook "/Game/Sprites/GreenZombie/GreenZombieWalk.GreenZombieWalk")
  (`PaperFlipbookComponent.SetLooping` _paperflipbook true)
  (`PaperFlipbookComponent.Play` _paperflipbook)
  (`PaperFlipbookComponent.SetPlayRate` _paperflipbook (`KismetMathLibrary.MapRangeClamped` (/ (`KismetMathLibrary.VSize` DistanceWalkedThisFrame) DeltaSeconds) (`self.WalkSpeed`) (`self.RunSpeed`) 1.0 2.0)))

(event `self.ZombieAttack`
  (params (DeltaSeconds :type "Float (single-precision)"))
  (bind _paperflipbook (`self.PaperFlipbook`))
  (`PaperFlipbookComponent.SetFlipbook` _paperflipbook "/Game/Sprites/GreenZombie/GreenZombieAttack.GreenZombieAttack")
  (`PaperFlipbookComponent.SetLooping` _paperflipbook false)
  (`PaperFlipbookComponent.PlayFromStart` _paperflipbook)
  (`PaperFlipbookComponent.SetPlayRate` _paperflipbook 1.0))

(fn `UserConstructionScript`)